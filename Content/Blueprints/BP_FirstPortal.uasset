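; BP_FirstPortal is a portal actor with a SceneCaptureComponent2D, apparently an early or unfinished attempt at a player-relative portal view.
; BeginPlay caches the player character, the actor transform and the capture component's initial rotation.
; A disconnected chain would aim the capture along the player-to-portal direction, mirrored in X and Y with pitch clamped.
; Tick is empty, so the capture never rotates at runtime.
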(event `self.ReceiveBeginPlay`
  (set `self.PlayerCharacterReference` (`GameplayStatics.GetPlayerCharacter` 0))
  (set `self.CurrentTransform` (`self.GetTransform` self))
  (set `self.InitialRotation` (`SceneComponent.K2_GetComponentRotation` (`self.SceneCaptureComponent2D`))))

(event `self.ReceiveTick`
  (params (DeltaSeconds :type "Float (single-precision)")))

(fn `UserConstructionScript`)